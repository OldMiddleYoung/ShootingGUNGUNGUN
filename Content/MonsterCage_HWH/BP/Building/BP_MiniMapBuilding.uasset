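; Minimap stand-in for a building that shows a beacon light according to the sign state of its referenced building.
; Tick copies BuildingSignState from BuildingRef while valid, then attaches either the escape point or normal mark-light particle to the Building component for the Escape Point or Select state.
; Spawning sets IsSelect, which stops further polling, so the beacon is not updated afterwards.
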(event `self.ReceiveTick`
  (params (DeltaSeconds :type "Float (single-precision)"))
  (if (not (`self.IsSelect`))
    (`/Engine/EditorBlueprintResources/StandardMacros.IsValid` (`self.BuildingRef`)
      (:`Is Valid`
        (set `self.BuildingSignState` (`/Game/MonsterCage_HWH/BP/Building/BP_BuildingBase.BuildingSignState` (`self.BuildingRef`))))
      (:`Is Not Valid`
        _))
    (switch `/Game/MonsterCage_HWH/BP/Data/Enum/E_BuildingSignState` (`self.BuildingSignState`)
      (:`NewEnumerator1`
        (`self.SpawnEscapeBeacon`))
      (:`NewEnumerator2`
        (`self.SpawnNormalBeacon`)))))

(event `SpawnEscapeBeacon`
  ;[1 1 1] SignFXFunction
  (`GameplayStatics.SpawnEmitterAttached` "/Game/MonsterCage_HWH/BP/VFX/P_MarkLight_EascapePoint.P_MarkLight_EascapePoint" (`self.Building`) "None" (0.0 0.0 -200.0))
  (set `self.IsSelect` true))

(event `SpawnNormalBeacon`
  ;[1 1 1] SignFXFunction
  (`GameplayStatics.SpawnEmitterAttached` "/Game/MonsterCage_HWH/BP/VFX/P_MarkLight_Normal.P_MarkLight_Normal" (`self.Building`) "None" (0.0 0.0 -50.0))
  (set `self.IsSelect` true))

(fn `UserConstructionScript`)