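; BP_BuildingBase is a placeholder-style building actor that can be marked as selected or as an escape point.
; Its construction script randomizes scale and base color through a dynamic material, then raises the mesh by its height to keep it grounded.
; Events switch the building's sign state.
; Eight seconds after BeginPlay, a building in the EscapePoint state spawns a BPA_EscapePoint at the Box1 transform.
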(event `SelectThisBuilding`
  (switch `/Game/MonsterCage_HWH/BP/Data/Enum/E_BuildingSignState` (`self.BuildingSignState`)
    (:`NewEnumerator0`
      (set `self.BuildingSignState` "NewEnumerator2"))))

(event `SelectThisBuildingAsEscapePoint`
  (set `self.BuildingSignState` "NewEnumerator1"))

(event `self.ReceiveBeginPlay`
  (`KismetSystemLibrary.Delay` 8.0)
  (switch `/Game/MonsterCage_HWH/BP/Data/Enum/E_BuildingSignState` (`self.BuildingSignState`)
    (:`NewEnumerator1`
      (`self.SpawnEscapePoint`))))

(event `SpawnEscapePoint`
  (`|SpawnActorFromClass` "/Game/MonsterCage_HWH/BP/EscapePoint/BPA_EscapePoint.BPA_EscapePoint_C" (`SceneComponent.K2_GetComponentToWorld` (`self.Box1`)) "Undefined" "OverrideRootScale" null null))

(fn `UserConstructionScript`
  (bind (_returnvalue_x _returnvalue_y _returnvalue_z) (`KismetMathLibrary.BreakVector` (`SceneComponent.K2_GetComponentScale` (`self.Building`))))
  (bind _returnvalue (`KismetMathLibrary.RandomFloatInRange` (`self.ScaleRangeMin_PH`) (`self.ScaleRangMax_PH`)))
  (`SceneComponent.SetWorldScale3D` (`self.Building`) (`KismetMathLibrary.MakeVector` _returnvalue _returnvalue (`KismetMathLibrary.RandomFloatInRange` (* (`self.ScaleRangeMin_PH`) (`self.ZMulti_Temp`)) (* (`self.ScaleRangMax_PH`) (`self.ZMulti_Temp`)))))
  (bind _returnvalue_2 (`PrimitiveComponent.CreateDynamicMaterialInstance` (`self.Building`) 0 "/Game/MonsterCage_HWH/MAt/M_Base.M_Base" "None"))
  (bind _output_get (set `self.MI` _returnvalue_2))
  (`MaterialInstanceDynamic.SetVectorParameterValue` _output_get "BaseColor" (make `LinearColor` (`KismetMathLibrary.RandomFloatInRange` 0.0 1.0) (`KismetMathLibrary.RandomFloatInRange` 0.0 1.0) (`KismetMathLibrary.RandomFloatInRange` 0.0 1.0)))
  (`SceneComponent.K2_SetRelativeLocation` (`self.Building`) (`KismetMathLibrary.MakeVector` 0.0 0.0 (* _returnvalue_z 50.0)) false false))