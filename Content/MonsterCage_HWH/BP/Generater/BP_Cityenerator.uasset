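; City generator actor that lays out a 3x3 grid of tile actors around its own location at BeginPlay.
; GenerateTheTile picks one random cell for a BP_TileBase_LandMark and fills every other cell with BP_TileBase.
; Tiles spawn at a fixed spacing offset from the generator's position along X and Y, at its height.
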(event `self.ReceiveBeginPlay`
  (set `self.LandMarker_X_Temp` (`KismetMathLibrary.RandomIntegerInRange` 0 2))
  (set `self.LandMarker_Y_Temp` (`KismetMathLibrary.RandomIntegerInRange` 0 2))
  (for _index (range 3)
    (for _index_2 (range 3)
      (if (== (`self.LandMarker_X_Temp`) _index)
        (if (== (`self.LandMarker_Y_Temp`) _index_2)
          (bind _returnvalue (`KismetMathLibrary.MakeVector` (+ (* _index 3500.0) (.x (`self.K2_GetActorLocation` self))) (+ (* _index_2 3500.0) (.y (`self.K2_GetActorLocation` self))) (.z (`self.K2_GetActorLocation` self))))
          (`|SpawnActorFromClass` "/Game/MonsterCage_HWH/BP/Tile/BP_TileBase_LandMark.BP_TileBase_LandMark_C" (`KismetMathLibrary.MakeTransform` _returnvalue) "Undefined" "OverrideRootScale" null null)
          (else
            (`|SpawnActorFromClass` "/Game/MonsterCage_HWH/BP/Tile/BP_TileBase.BP_TileBase_C" (`KismetMathLibrary.MakeTransform` _returnvalue) "Undefined" "OverrideRootScale" null null :!label _label)))
        (else
          (goto _label))))))

(fn `UserConstructionScript`)