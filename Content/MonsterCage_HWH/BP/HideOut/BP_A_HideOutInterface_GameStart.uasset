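; A hideout interactable that starts a game run when the player uses it.
; Overlapping its confirm area shows its name and registers it as the player character's interaction target, with a placeholder on-screen debug prompt.
; On interaction it calls ChangeLevel on the first BP_warehouse in the world, then saves the player's backpack items into the game instance.
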(event `self.ReceiveTick`
  (params (DeltaSeconds :type "Float (single-precision)"))
  ;[1 1 1] PlaceHolderFunction
  (if (`self.ShowDebugInfo`)
    (`KismetSystemLibrary.PrintString` "Press\"A\" to start game" true true (struct :`G` 0.66 :`B` 1.0 :`A` 1.0) 0.0)))

(event `self.ConfirmArea.OnComponentBeginOverlap`
  (params (OverlappedComponent :type "PrimitiveComponent Object Reference") (OtherActor :type "Actor Object Reference") (OtherComp :type "PrimitiveComponent Object Reference") (OtherBodyIndex :type Integer) (bFromSweep :type Boolean) (SweepResult :type "HitResult Structure (by ref)"))
  (bind _asbp_player_main_character (cast `/Game/TST_ZAP/BluePrint_ZAP/BP_PlayerMainCharacter` OtherActor))
  (`self.ShowName`)
  (set `self.ShowDebugInfo` true)
  (set `/Game/TST_ZAP/BluePrint_ZAP/BP_PlayerMainCharacter.InterActionStuff` self _asbp_player_main_character))

(event `self.ConfirmArea.OnComponentEndOverlap`
  (params (OverlappedComponent :type "PrimitiveComponent Object Reference") (OtherActor :type "Actor Object Reference") (OtherComp :type "PrimitiveComponent Object Reference") (OtherBodyIndex :type Integer))
  (bind _asbp_player_main_character (cast `/Game/TST_ZAP/BluePrint_ZAP/BP_PlayerMainCharacter` OtherActor))
  (`self.UnShowName`)
  (set `self.ShowDebugInfo` false)
  (set `/Game/TST_ZAP/BluePrint_ZAP/BP_PlayerMainCharacter.InterActionStuff` null _asbp_player_main_character))

(event `/Game/MonsterCage_HWH/BP/Interface/BPI_Interaction.Interaction`
  (bind _outactors (`GameplayStatics.GetAllActorsOfClass` "/Game/MonsterCage_HWH/BP/HideOut/BP_warehouse.BP_warehouse_C"))
  (`/Game/MonsterCage_HWH/BP/HideOut/BP_warehouse.ChangeLevel` (`|GetArrayItem` _outactors))
  (bind _asbp_ggggame_instance (cast `/Game/MonsterCage_HWH/BP/BP_GGGGameInstance` (`GameplayStatics.GetGameInstance`)))
  (bind _asbp_player_main_character (cast `/Game/TST_ZAP/BluePrint_ZAP/BP_PlayerMainCharacter` (`GameplayStatics.GetPlayerPawn` 0)))
  (`/Game/MonsterCage_HWH/BP/BP_GGGGameInstance.SaveItemInBag` _asbp_ggggame_instance (`/Game/TST_ZZ/Pack/Packcomp.pack_array` (`/Game/TST_ZAP/BluePrint_ZAP/BP_PlayerMainCharacter.Packcomp` _asbp_player_main_character))))

(fn `UserConstructionScript`
  (`parent.UserConstructionScript`))