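; BP_BigMapGameMode is the big map's game mode, which picks a random building as the escape point once city generation ends.
; Tick polls every BP_Cityenerator until all report finished, latching a completion flag.
; After a short delay, a DoOnce gathers all BP_BuildingBase actors and calls SelectThisBuildingAsEscapePoint on a random one.
; The random index is rolled separately for the validity check and the call, so they can hit different buildings.
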(event `self.ReceiveTick`
  (params (DeltaSeconds :type "Float (single-precision)"))
  (`|ExecutionSequence`
    (:`then_0`
      (if (not (`self.IsAllGeneratorFinishedSpawn`))
        (set `self.IsAllGeneratorFinishedSpawn` true)
        (bind _outactors (`GameplayStatics.GetAllActorsOfClass` "/Game/MonsterCage_HWH/BP/Generater/BP_Cityenerator.BP_Cityenerator_C"))
        (for _array_element _outactors
          (if (not (`/Game/MonsterCage_HWH/BP/Generater/BP_Cityenerator.FinishedGenerator` _array_element))
            (set `self.IsAllGeneratorFinishedSpawn` false)
            (break)))))
    (:`then_1`
      (`KismetSystemLibrary.Delay` 3.0)
      (if (`self.IsAllGeneratorFinishedSpawn`)
        (`/Engine/EditorBlueprintResources/StandardMacros.DoOnce` false
          (:`Completed`
            (bind _outactors_2 (`GameplayStatics.GetAllActorsOfClass` "/Game/MonsterCage_HWH/BP/Building/BP_BuildingBase.BP_BuildingBase_C"))
            (bind _output_get (set `self.BuildingArray` _outactors_2))
            (bind _output (`|GetArrayItem` _output_get (`KismetMathLibrary.RandomIntegerInRange` 0 (- (`KismetArrayLibrary.Array_Length` _output_get) 1))))
            (`/Engine/EditorBlueprintResources/StandardMacros.IsValid` _output
              (:`Is Valid`
                (`/Game/MonsterCage_HWH/BP/Building/BP_BuildingBase.SelectThisBuildingAsEscapePoint` _output)))))))))

(fn `UserConstructionScript`)