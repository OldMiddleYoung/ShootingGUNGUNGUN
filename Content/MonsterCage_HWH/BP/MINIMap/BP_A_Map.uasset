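; 3D minimap actor that shows a scaled-down copy of the city and follows the player's MapPos component every tick.
; On BeginPlay it copies each BP_Cityenerator's buildings as attached BP_MiniMapBuilding actors, with a separate material for landmarks, then hides itself at zero scale.
; ShowMap and UnShowMap play or reverse a scale timeline, and a spring arm takes yaw offsets for map camera rotation.
; The construction script sizes the ground from the tile counts and scale.
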(event `self.ReceiveTick`
  (params (DeltaSeconds :type "Float (single-precision)"))
  ;[1 1 1] UpadteLocation
  (bind _asbp_player_main_character (cast `/Game/TST_ZAP/BluePrint_ZAP/BP_PlayerMainCharacter` (`GameplayStatics.GetPlayerPawn` 0)))
  (`self.K2_SetActorLocation` (`SceneComponent.K2_GetComponentLocation` (`/Game/TST_ZAP/BluePrint_ZAP/BP_PlayerMainCharacter.MapPos` _asbp_player_main_character))))

(event `self.ReceiveBeginPlay`
  (bind _scaletimes (`self.ScaleTimes`))
  (bind (_buildinginfo_temp_buildingmesh _buildinginfo_temp_buildingmeshscale_p) (break `/Game/MonsterCage_HWH/BP/Data/Structure/S_BuildingInfo` (`self.BuildingInfo_temp`)))
  (bind (_buildinginfo_temp_buildingmesh_2 _buildinginfo_temp_buildingmeshscale_p_2 _buildinginfo_temp_relativelocation _buildinginfo_temp_islandmark) (break `/Game/MonsterCage_HWH/BP/Data/Structure/S_BuildingInfo` (`self.BuildingInfo_temp`)))
  (bind (_buildinginfo_temp_buildingmesh_3 _buildinginfo_temp_buildingmeshscale_p_3 _buildinginfo_temp_relativelocation_2 _buildinginfo_temp_islandmark_2 _buildinginfo_temp_buildingref) (break `/Game/MonsterCage_HWH/BP/Data/Structure/S_BuildingInfo` (`self.BuildingInfo_temp`)))
  ;[1 1 1] Initial
  (`|ExecutionSequence`
    (:`then_0`
      (bind _outactors (`GameplayStatics.GetAllActorsOfClass` "/Game/MonsterCage_HWH/BP/Generater/BP_Cityenerator.BP_Cityenerator_C"))
      (bind _output_get (set `self.GeneratorArray` _outactors))
      (for _array_element _output_get
        (for _array_element_2 (`/Game/MonsterCage_HWH/BP/Generater/BP_Cityenerator.BuildingArray` _array_element)
          (bind _output_get_2 (set `self.BuildingInfo_temp` _array_element_2))
          (bind _returnvalue_location (`KismetMathLibrary.BreakTransform` (`KismetMathLibrary.MakeRelativeTransform` (`self.GetTransform` _array_element) (`self.GetTransform` (`self.BasicTile`)))))
          (bind _returnvalue (`|SpawnActorFromClass` "/Game/MonsterCage_HWH/BP/Building/BP_MiniMapBuilding.BP_MiniMapBuilding_C" (`KismetMathLibrary.MakeTransform` (+ (* (`.RelativeLocation_5_37FC38FB4A3F58FC455D22AC4C1E847F` (break `/Game/MonsterCage_HWH/BP/Data/Structure/S_BuildingInfo` _output_get_2)) (`self.MultiTimes`)) (* _returnvalue_location (`self.MultiTimes`)) (`self.K2_GetActorLocation`) (`KismetMathLibrary.MakeVector` (* _scaletimes -100.0) (* _scaletimes -100.0))) (struct) (* _buildinginfo_temp_buildingmeshscale_p (`self.MultiTimes`))) "Undefined" "OverrideRootScale" null null))
          (`self.K2_AttachToActor` _returnvalue self "None" "KeepWorld" "KeepWorld" "KeepWorld" true)
          (set `/Game/MonsterCage_HWH/BP/Building/BP_MiniMapBuilding.BuildingRef` _buildinginfo_temp_buildingref _returnvalue)
          (`KismetArrayLibrary.Array_Add` (`self.MiniMapBuildingArray`) _returnvalue)
          (bind _building (`/Game/MonsterCage_HWH/BP/Building/BP_MiniMapBuilding.Building` _returnvalue))
          (`StaticMeshComponent.SetStaticMesh` _building _buildinginfo_temp_buildingmesh_2)
          (if _buildinginfo_temp_islandmark
            (`PrimitiveComponent.SetMaterial` _building 0 "/Game/MonsterCage_HWH/MAt/M_Base_MinimapLandmark.M_Base_MinimapLandmark")
            (else
              (`PrimitiveComponent.SetMaterial` _building 0 "/Game/MonsterCage_HWH/MAt/M_Base_MiniMapBuildingBase.M_Base_MiniMapBuildingBase"))))))
    (:`then_1`
      (`self.SetActorScale3D` (0.0 0.0 0.0)))))

(event `AddCameraRotationOffset`
  (params (Value :type "Float (double-precision)"))
  ;[1 1 1] MapCameraRotation
  (`SceneComponent.K2_AddWorldRotation` (`self.SpringArm`) (`KismetMathLibrary.MakeRotator` 0.0 0.0 Value) false false))

(event `ShowMap`
  ;[1 1 1] Show&UnShow Map
  (if (`self.IsShowMapTimeLineFinished`)
    (set `self.IsShowMapTimeLineFinished` false)
    (bind (_direction _scale) (`Timeline|ShowMapTimeline` :!label _label)
      (:`Update`
        (`self.SetActorScale3D` (`KismetMathLibrary.MakeVector` _scale _scale _scale)))
      (:`Finished`
        (set `self.IsShowMapTimeLineFinished` true)))))

(event `UnShowMap`
  ;[1 1 1] Show&UnShow Map
  (if (`self.IsShowMapTimeLineFinished`)
    (set `self.IsShowMapTimeLineFinished` false)
    (goto _label :!via `Reverse`)))

(fn `UserConstructionScript`
  (set `self.ScaleTimes` (* (`self. TileScale`) (`self.MultiTimes`)))
  (`SceneComponent.SetWorldScale3D` (`self.Ground`) (`KismetMathLibrary.MakeVector` (+ (* (`KismetMathLibrary.Conv_IntToDouble` (`self.NUM_X`)) (`self.ScaleTimes`)) 0.02) (+ (* (`KismetMathLibrary.Conv_IntToDouble` (`self.NUM_Y`)) (`self.ScaleTimes`)) 0.02) 0.05)))