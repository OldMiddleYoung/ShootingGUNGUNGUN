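; BP_logic_exp is a short-lived explosion actor that spawns the P_Explosion particle effect at its location and destroys itself after a brief delay.
; While it lives, Tick grows a Radius value at a constant rate and applies it to the ExpLogic sphere, updating overlaps as it expands.
; The sphere's begin-overlap event is empty, so the expanding volume triggers no response within this Blueprint.
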(event `self.ReceiveBeginPlay`
  (`GameplayStatics.SpawnEmitterAtLocation` "/Game/TST_ZZ/VFX_import/CartoonyImpact2/Particles/P_Explosion.P_Explosion" (`SceneComponent.K2_GetComponentLocation` (`self.DefaultSceneRoot`)))
  (`KismetSystemLibrary.Delay` 0.4)
  (`self.K2_DestroyActor`))

(event `self.ReceiveTick`
  (params (DeltaSeconds :type "Float (single-precision)"))
  (bind _output_get (set `self.radius` (+ (* DeltaSeconds 400.0) (`self.radius`))))
  (`SphereComponent.SetSphereRadius` (`self.exp_logic`) _output_get true))

(event `self.exp_logic.OnComponentBeginOverlap`
  (params (OverlappedComponent :type "PrimitiveComponent Object Reference") (OtherActor :type "Actor Object Reference") (OtherComp :type "PrimitiveComponent Object Reference") (OtherBodyIndex :type Integer) (bFromSweep :type Boolean) (SweepResult :type "HitResult Structure (by ref)")))

(fn `UserConstructionScript`)