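; BP_grenade is a grenade actor that explodes on contact.
; An overlap on its Capsule component calls the exp event, which spawns BP_logic_exp at the Vectorhelper component's world location and then destroys the grenade.
; The spawn ignores collisions, and the graph holds no movement, timer or damage logic of its own.
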(event `self.Capsule.OnComponentBeginOverlap`
  (params (OverlappedComponent :type "PrimitiveComponent Object Reference") (OtherActor :type "Actor Object Reference") (OtherComp :type "PrimitiveComponent Object Reference") (OtherBodyIndex :type Integer) (bFromSweep :type Boolean) (SweepResult :type "HitResult Structure (by ref)"))
  (`self.exp`))

(event `exp`
  (`|SpawnActorFromClass` "/Game/TST_ZZ/weapons/individual/BP_logic_exp.BP_logic_exp_C" (`KismetMathLibrary.MakeTransform` (`SceneComponent.K2_GetComponentLocation` (`self.vectorhelper`))) "AlwaysSpawn" "OverrideRootScale" null null)
  (`self.K2_DestroyActor`))

(fn `UserConstructionScript`
  (`parent.UserConstructionScript`))