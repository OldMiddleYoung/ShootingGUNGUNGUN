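; Base gun actor that fires projectiles from a spawn point, with switchable burst modes and optional hold-to-fire, bound to gamepad triggers and shoulders.
; Input sets InputStack to the current mode's shot count, or -1 for continuous fire until release.
; Tick runs down the cooldown and fires while the stack is nonzero, decrementing it after each shot's delay.
; Animation and FX events are empty override hooks.
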(event `hold_input_reset`
  ;[1 1 1] press input and hold input function
  (set `self.input_stack` 0))

(event `Key|Gamepad_RightTrigger`
  (params (Key :type "Key Structure"))
  ;[1 1 1] default input bond
  (:`Pressed`
    (`self.hold_input`))
  (:`Released`
    (`self.hold_input_reset`)))

(event `hold_input`
  ;[1 1 1] press input and hold input function
  (if (`self.holding_to_fire`)
    (set `self.input_stack` -1)
    (else
      (if (== (`self.input_stack`) 0) :!label _label
        (set `self.input_stack` (`|GetArrayItem` (`self.shooting_mode_array`) (`self.shoot_mode_pointer`)))))))

(event `Key|Gamepad_RightShoulder`
  (params (Key :type "Key Structure"))
  ;[1 1 1] default input bond
  (:`Pressed`
    (`self.press_input`)))

(event `press_input`
  ;[1 1 1] press input and hold input function
  (goto _label))

(event `Key|Gamepad_LeftShoulder`
  (params (Key :type "Key Structure"))
  ;[1 1 1] default input bond
  (:`Pressed`
    (`self.switch_mode`)))

(event `switch_mode`
  ;[1 1 1] switch mode function 1tap 3tap etc
  (`/Engine/EditorBlueprintResources/StandardMacros.IncrementInt` (`self.shoot_mode_pointer`)
    (:`  `
      (set `self.shoot_mode_pointer` (mod (`self.shoot_mode_pointer`) (`KismetArrayLibrary.Array_Length` (`self.shooting_mode_array`)))))))

(event `self.ReceiveTick`
  (params (DeltaSeconds :type "Float (single-precision)"))
  ;[1 1 1] tick
  (bind _output_get (set `self.cooldown_instance` (- (`self.cooldown_instance`) DeltaSeconds)))
  (if (<= _output_get 0.0)
    (set `self.cooldown_instance` 0.0)
    (if (!= (`self.input_stack`) 0)
      (`self.shoot_single`))))

(event `shoot_single`
  ;[1 1 1] 1 shoot
  (`self.playFX`)
  (`self.playAnim`)
  (`self.spawn_bullet_in_one_shoot`)
  (set `self.cooldown_instance` (`self.one_bullet_cooldown`))
  (`KismetSystemLibrary.Delay` (`self.one_bullet_cooldown`))
  (`/Engine/EditorBlueprintResources/StandardMacros.DecrementInt` (`self.input_stack`)))

(event `spawn_bullet_in_one_shoot`
  ;[1 1 1] default spawn
  (`|SpawnActorFromClass` (`self.bullet_type`) (`SceneComponent.K2_GetComponentToWorld` (`self.spawnpoint`)) "AdjustIfPossibleButAlwaysSpawn" "OverrideRootScale" null null))

(event `playAnim`
  ;[1 1 1] override
)

(event `playFX`
  ;[1 1 1] override
)

(fn `UserConstructionScript`)