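; BP_Character_Basic is a base character with sprinting, stick-driven aiming, health and death.
; For players, Tick arbitrates sprint and aim states, which set walk speed, rotation mode and aim-ray visibility, while RotateChar eases control rotation toward the aim stick.
; beHited plays a random damage montage, subtracts BPCMPDemageCaculater's result, updates a camera-facing 3D health bar and triggers Death at zero.
; Overlap-driven hits and shooting speed control are left unwired.
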(event `Shooting Start`
  ;[1 0.7968 0.2917] Archived
  ;;[1 1 1] AimController
  ;;;[1 0 0] Shooting Controller_Basic event(Not use)
  (`self.SprintEnd`)
  (set `CharacterMovementComponent.MaxWalkSpeed` 150.0 (`self.CharacterMovement`)))

(event `self.ReceiveTick`
  (params (DeltaSeconds :type "Float (single-precision)"))
  (bind _healthposition (`self.HealthPosition`))
  ;[1 0.7968 0.2917] Archived
  ;;[1 1 1] TickTime
  (set `self.TickTime` DeltaSeconds)
  (`|ExecutionSequence`
    (:`then_0`
      ;;[1 1 1] AimController
      (if (`self.isPlayer`)
        (if (`self.Sprint Button Down`)
          ;;;[1 1 1] SprintController
          (if (<= (`KismetMathLibrary.VSize` (`self.StickMoveVector`)) 0.6)
            (`self.SprintEnd`)
            (elif (`self.isShooting`)
              (`self.SprintEnd`)
              (else
                ;;;[1 1 1] AimController_1
                (if (`self.IsAiming`)
                  (`self.SprintEnd`)
                  (`self.Aiming Start`)))))
          (else
            ;;;[1 1 1] AimController_0
            (if (`self.IsAiming`)
              (`self.Aiming Start`)
              (else
                (`self.Aiming End`)))))))
    (:`then_1`
      ;[1 1 1] Initial UI rotation
      (`SceneComponent.K2_SetWorldRotation` _healthposition (`KismetMathLibrary.FindLookAtRotation` (`SceneComponent.K2_GetComponentLocation` _healthposition) (`SceneComponent.K2_GetComponentLocation` (`self.CameraPos`))) false false))))

(event `Shooting End`
  ;[1 0.7968 0.2917] Archived
  ;;[1 1 1] AimController
  ;;;[1 0 0] Shooting Controller_Basic event(Not use)
  (set `CharacterMovementComponent.MaxWalkSpeed` 300.0 (`self.CharacterMovement`)))

(event `Aiming Start`
  ;[1 0.7968 0.2917] Archived
  ;;[1 1 1] AimController
  ;;;[1 1 1] Aiming Controller_Basic event
  (set `CharacterMovementComponent.bOrientRotationToMovement` false (`self.CharacterMovement`))
  (set `CharacterMovementComponent.MaxWalkSpeed` 150.0 (`self.CharacterMovement`))
  (`SceneComponent.SetVisibility` (`self.TargetRay`) true false))

(event `Aiming End`
  ;[1 0.7968 0.2917] Archived
  ;;[1 1 1] AimController
  ;;;[1 1 1] Aiming Controller_Basic event
  (set `CharacterMovementComponent.bOrientRotationToMovement` true (`self.CharacterMovement`))
  (set `CharacterMovementComponent.MaxWalkSpeed` 300.0 (`self.CharacterMovement`))
  (`SceneComponent.SetVisibility` (`self.TargetRay`) false false))

(event `RotateChar`
  (bind _stickaimvector (`self.StickAimVector`))
  (bind _returnvalue (`SceneComponent.K2_GetComponentRotation` (`self.CapsuleComponent`)))
  ;[1 0.7968 0.2917] Archived
  ;;[1 1 1] Rotation Controller
  ;;;[1 1 1] Rotate Char
  (if (not (`self.Sprint Button Down`))
    (if (`self.IsAiming`)
      (`Controller.SetControlRotation` (`self.GetController`) (`KismetMathLibrary.RLerp` _returnvalue (`KismetMathLibrary.RInterpTo` _returnvalue (`KismetMathLibrary.MakeRotator` 0.0 0.0 (+ (.yaw (`KismetMathLibrary.Conv_VectorToRotator` _stickaimvector)) 90.0)) (`self.TickTime`) (`self.MiddleLerpSpeed`)) (* (`KismetMathLibrary.FMax` (`KismetMathLibrary.Abs` (.x _stickaimvector)) (`KismetMathLibrary.Abs` (.y _stickaimvector))) (`self.FinalLerpSpeedDegree`)) true)))))

(event `SprintBegin`
  ;[1 0.7968 0.2917] Archived
  ;;[1 1 1] SprintController
  ;;;[1 1 1] Sprint
  (set `self.Sprint Button Down` true)
  (set `CharacterMovementComponent.MaxWalkSpeed` 750.0 (`self.CharacterMovement`)))

(event `SprintEnd`
  ;[1 0.7968 0.2917] Archived
  ;;[1 1 1] SprintController
  ;;;[1 1 1] Run
  (set `self.Sprint Button Down` false)
  (set `CharacterMovementComponent.MaxWalkSpeed` 300.0 (`self.CharacterMovement`)))

(event `self.ReceiveBeginPlay`
  ;[1 1 1] InilitialTheHP
  (set `self.CurrentHealthPoint` (`self.MaxHealthPoint`)))

(event `self.CapsuleComponent.OnComponentBeginOverlap`
  (params (OverlappedComponent :type "PrimitiveComponent Object Reference") (OtherActor :type "Actor Object Reference") (OtherComp :type "PrimitiveComponent Object Reference") (OtherBodyIndex :type Integer) (bFromSweep :type Boolean) (SweepResult :type "HitResult Structure (by ref)"))
  ;[1 1 1] hitController
)

(event `beHited`
  (params (hitedActor :type "Actor Object Reference"))
  ;[1 1 1] BeHited
  (`|ExecutionSequence`
    (:`then_0`
      (`AnimInstance.Montage_Play` (`SkeletalMeshComponent.GetAnimInstance` (`self.Mesh`)) (`|GetArrayItem` (`self.DamagedMontage`) (`KismetMathLibrary.RandomInteger` 4)) 1.0 "MontageLength" 0.0 true))
    (:`then_1`
      (bind _truedamage (`/Game/TST_ZAP/BasicClass/BP_CMP_DemageCaculater.Caculater` (`self.BP_CMP_DemageCaculater`) hitedActor))
      (bind _output_get (set `self.CurrentHealthPoint` (- (`self.CurrentHealthPoint`) _truedamage)))
      (`|ExecutionSequence`
        (:`then_0`
          (if (<= _output_get 0.0)
            (set `self.CurrentHealthPoint` 0.0)
            (`self.Death`)))
        (:`then_1`
          ;[1 1 1] UI
          (bind _asbp_3dui (cast `/Game/TST_ZAP/UI/BP_3DUI` (`WidgetComponent.GetUserWidgetObject` (`self.HealthPosition`))))
          (`ProgressBar.SetPercent` (`/Game/TST_ZAP/UI/BP_3DUI.HealthBar` _asbp_3dui) (/ (`self.CurrentHealthPoint`) (`self.MaxHealthPoint`))))))))

(event `Death`
  ;[1 1 1] Death
  (`|ExecutionSequence`
    (:`then_0`
      (`self.SetActorEnableCollision` false))
    (:`then_1`
      (`AnimInstance.Montage_Play` (`SkeletalMeshComponent.GetAnimInstance` (`self.Mesh`)) (`|GetArrayItem` (`self.DeathMontage`) (`KismetMathLibrary.RandomInteger` 3)) 1.0 "MontageLength" 0.0 true))))

(fn `UserConstructionScript`)